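; Ocean water actor that damages the player while they are inside its Waterdamage volume.
; Overlap begin sets PlayerInWater and starts a Delay-based loop that repeatedly subtracts a small amount from PlayerOne's PlayerHealth.
; The loop calls Death on player character 0 once health runs out.
; Overlap end clears the flag, which stops the loop at its next check after the delay.
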(event `self.Waterdamage.OnComponentBeginOverlap`
  (params (OverlappedComponent :type "PrimitiveComponent Object Reference") (OtherActor :type "Actor Object Reference") (OtherComp :type "PrimitiveComponent Object Reference") (OtherBodyIndex :type Integer) (bFromSweep :type Boolean) (SweepResult :type "HitResult Structure (by ref)"))
  (bind _asplayer_one (cast `/Game/Blueprints/ThirdPersonBP/Blueprints/PlayerOne` OtherActor))
  (set `self.PlayerInWater` true)
  (bind _output_get (set `/Game/Blueprints/ThirdPersonBP/Blueprints/PlayerOne.PlayerHealth` (- (`/Game/Blueprints/ThirdPersonBP/Blueprints/PlayerOne.PlayerHealth` _asplayer_one) 0.1) _asplayer_one :!label _label))
  (if (<= _output_get 0.0)
    (bind _asplayer_one_2 (cast `/Game/Blueprints/ThirdPersonBP/Blueprints/PlayerOne` (`GameplayStatics.GetPlayerCharacter` 0)))
    (`/Game/Blueprints/ThirdPersonBP/Blueprints/PlayerOne.Death` _asplayer_one_2)
    (else
      (`KismetSystemLibrary.Delay` 1.5)
      (if (`self.PlayerInWater`)
        (goto _label)))))

(event `self.Waterdamage.OnComponentEndOverlap`
  (params (OverlappedComponent :type "PrimitiveComponent Object Reference") (OtherActor :type "Actor Object Reference") (OtherComp :type "PrimitiveComponent Object Reference") (OtherBodyIndex :type Integer))
  (cast `/Game/Blueprints/ThirdPersonBP/Blueprints/PlayerOne` OtherActor)
  (set `self.PlayerInWater` false))

(fn `UserConstructionScript`)