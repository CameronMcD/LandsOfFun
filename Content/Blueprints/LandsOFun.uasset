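; LandsOFun is a Blueprint that runs a minutes-and-seconds countdown and ends play when time runs out.
; Tick feeds a one-second Delay, so Seconds drops about once per second and rolls over into Minutes below zero.
; Once Minutes goes negative, it creates the TIMESUP widget, adds it to the viewport and pauses the game.
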(event `self.ReceiveTick`
  (params (DeltaSeconds :type "Float (single-precision)"))
  ;[1 1 1] Variable Minutes And Seconds are called to create timer
  (`KismetSystemLibrary.Delay` 1.0)
  (set `self.Seconds` (- (`self.Seconds`) 1))
  (if (< (`self.Seconds`) 0)
    (set `self.Minutes` (- (`self.Minutes`) 1))
    (set `self.Seconds` 59))
  (if (<= (`self.Minutes`) -1)
    (bind _returnvalue (`|CreateWidget` "/Game/Blueprints/TIMESUP.TIMESUP_C"))
    (`UserWidget.AddToViewport` _returnvalue 0)
    (`GameplayStatics.SetGamePaused` true)))

(fn `UserConstructionScript`)